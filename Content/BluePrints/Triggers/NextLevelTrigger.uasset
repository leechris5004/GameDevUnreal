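; Level transition trigger that loads the next level when the Antoine player character overlaps it.
; On overlap it fades the camera and audio out, removes all widgets and resets the save point and spawn position stored in the Global game instance.
; After a delay matching the fade, it opens the level named by its Level variable.
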(event `self.ReceiveActorBeginOverlap`
  (params (OtherActor :type "Actor Object Reference"))
  ;[1 1 1] If player enters trigger, move to next level
  (if (`KismetMathLibrary.ClassIsChildOf` (`GameplayStatics.GetObjectClass` OtherActor) "/Game/BluePrints/Antoine.Antoine_C")
    (`PlayerCameraManager.StartCameraFade` :`self` (`GameplayStatics.GetPlayerCameraManager` 0) :`ToAlpha` 1.0 :`Duration` 1.0 :`bShouldFadeAudio` true :`bHoldWhenFinished` true)
    (`WidgetLayoutLibrary.RemoveAllWidgets`)
    (bind _asglobal (cast `/Game/BluePrints/Global` (`GameplayStatics.GetGameInstance`)))
    (set `/Game/BluePrints/Global.SavePoint` 0 _asglobal)
    (set `/Game/BluePrints/Global.SpawnPosition` (0.0 0.0 0.0) _asglobal)
    (`KismetSystemLibrary.Delay` 1.0)
    (`GameplayStatics.OpenLevel` (`self.Level`))))

(fn `UserConstructionScript`)