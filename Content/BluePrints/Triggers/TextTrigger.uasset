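; TextTrigger is a trigger actor that shows a line of dialogue on screen when the Antoine character first walks into it.
; On BeginPlay it waits briefly for the level UI to load, then caches the first GameplayUI widget it finds.
; An overlap by Antoine clears a one-shot flag, writes the trigger's Text into the UI and plays its FadeText animation in ping-pong mode.
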(event `self.ReceiveBeginPlay`
  ;[1 1 1] Set UI to level UI. Delay is needed so the level UI loads first
  (`KismetSystemLibrary.Delay` 0.2)
  (bind _foundwidgets (`WidgetBlueprintLibrary.GetAllWidgetsOfClass` "/Game/BluePrints/UI/GameplayUI.GameplayUI_C" false))
  (set `self.UI` (`|GetArrayItem` _foundwidgets)))

(event `self.ReceiveActorBeginOverlap`
  (params (OtherActor :type "Actor Object Reference"))
  (bind _ui (`self.UI`))
  ;[1 1 1] Play the dialogue in the UI
  (if (and (`KismetMathLibrary.ClassIsChildOf` (`GameplayStatics.GetObjectClass` OtherActor) "/Game/BluePrints/Antoine.Antoine_C") (`self.Not Played`))
    (set `self.Not Played` false)
    (set `/Game/BluePrints/UI/GameplayUI.DialogueText` (`KismetTextLibrary.Conv_StringToText` (`self.Text`)) _ui)
    (`UserWidget.PlayAnimation` _ui (`/Game/BluePrints/UI/GameplayUI.FadeText` _ui) 0.0 1 "PingPong" 1.0)))

(fn `UserConstructionScript`)