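; A trigger actor that plays a named level sequence cutscene once when the Antoine character overlaps it.
; Shortly after BeginPlay it searches all LevelSequenceActors for one whose object name matches CutsceneName and stores it.
; On overlap it checks the actor's class and a NotPlayed flag, then clears the flag and starts the sequence player.
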(event `self.ReceiveBeginPlay`
  ;[1 1 1] Set Cutscene based on Name
  (`KismetSystemLibrary.Delay` 0.2)
  (bind _outactors (`GameplayStatics.GetAllActorsOfClass` "/Script/LevelSequence.LevelSequenceActor"))
  (for _array_element _outactors
    (if (== (`KismetSystemLibrary.GetObjectName` _array_element) (`self.Cutscene Name`))
      (set `self.Cutscene` _array_element)
      (break))))

(event `self.ReceiveActorBeginOverlap`
  (params (OtherActor :type "Actor Object Reference"))
  ;[1 1 1] Play Cutscene on overlap
  (if (and (`KismetMathLibrary.ClassIsChildOf` (`GameplayStatics.GetObjectClass` OtherActor) "/Game/BluePrints/Antoine.Antoine_C") (`self.Not Played`))
    (set `self.Not Played` false)
    (`MovieSceneSequencePlayer.Play` (`LevelSequenceActor.SequencePlayer` (`self.Cutscene`)))))

(fn `UserConstructionScript`)